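; Player character Blueprint whose only live logic toggles the pause menu from the IA_PauseGame input.
; Opening creates WBP_PauseMenu and sets Game and UI input, then after a short delay focuses Resume for keyboard navigation, shows the cursor and pauses.
; Pressing again removes the widget, unpauses and restores game-only input with a hidden cursor.
; A disconnected main-menu creation chain remains in the graph and never runs.
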(event Input|EnhancedActionEvents|EnhancedInputActionIA_PauseGame
  (params (ActionValue :type Boolean) (ElapsedSeconds :type Float%20%28double-precision%29) (TriggeredSeconds :type Float%20%28double-precision%29) (InputAction :type Input%20Action%20Object%20Reference :default "/Game/Blueprints/Characters/Input/IA_PauseGame.IA_PauseGame"))
  (bind _returnvalue (Game|GetPlayerController 0))
  (:Started
    (if (not (Variables|Default|GetIsPauseMenuOpen))
      (Variables|Default|SetIsPauseMenuOpen true)
      (bind _returnvalue_2 (Game|ConstructObjectfromClass _returnvalue "/Game/UI/WBP_PauseMenu.WBP_PauseMenu_C"))
      (bind _output_get (Variables|Default|SetPauseMenuWidget _returnvalue_2))
      (UserInterface|Viewport|AddtoViewport _output_get 0)
      (Input|SetInputModeGameandUI _returnvalue (Variables|Default|GetPauseMenuWidget) "DoNotLock" true false)
      (Utilities|FlowControl|Delay 0.2)
      (Widget|SetKeyboardFocus (Variables|/Game/UI/WBP_PauseMenu.WBP_PauseMenu_C|GetResumeButton _returnvalue_2))
      (Variables|/Script/Engine.PlayerController|SetbShowMouseCursor (Game|GetPlayerController 0) true)
      (Game|SetGamePaused true)
      (else
        (Variables|Default|SetIsPauseMenuOpen false)
        (Widget|RemovefromParent (Variables|Default|GetPauseMenuWidget))
        (Game|SetGamePaused false)
        (Input|SetInputModeGameOnly _returnvalue false)
        (Variables|/Script/Engine.PlayerController|SetbShowMouseCursor (Game|GetPlayerController 0) false)))))

(event Collision|EventActorBeginOverlap
  (params (OtherActor :type Actor%20Object%20Reference)))

(event EventTick
  (params (DeltaSeconds :type Float%20%28single-precision%29)))

(fn ConstructionScript)