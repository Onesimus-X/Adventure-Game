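; BP_CastleGate is a castle gate actor that opens once enough items have been collected.
; Each CollectItem event increments a counter, and reaching the maximum triggers OpenGate through a DoOnce so the gate opens only once.
; OpenGate runs a timeline that lerps the iron gate's relative height upward and plays a lift sound at the actor's location.
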(event Custom|OpenGate
  (Utilities|FlowControl|Sequence
    (:then_0
      (bind _gate_lift (Timeline|Open%20Gate%20Anim Play)
        (:Update
          (Transformation|SetRelativeLocation (Variables|Default|GetIronGate) (Math|Vector|MakeVector 0.0 0.0 (Math|Float|Lerp 147.0 5e+02 _gate_lift)) false false))))
    (:then_1
      (Audio|PlaySoundatLocation "/Game/Audio/GateLift_Cue.GateLift_Cue" (Transformation|GetActorLocation) "0, 0, 0" 1.0 1.0 0.0 0 0 0 0))))

(event Custom|Collect%20Item
  (Math|Integer|IncrementInt (Variables|Default|GetCurrentItemsCollected)
    (:%20%20
      (if (>= (Variables|Default|GetCurrentItemsCollected) (Variables|Default|GetMaxItemsCollected))
        (Utilities|FlowControl|DoOnce false
          (:Completed
            (CallFunction|OpenGate)))))))

(event Collision|EventActorBeginOverlap
  (params (OtherActor :type Actor%20Object%20Reference)))

(event EventTick
  (params (DeltaSeconds :type Float%20%28single-precision%29)))

(fn ConstructionScript)